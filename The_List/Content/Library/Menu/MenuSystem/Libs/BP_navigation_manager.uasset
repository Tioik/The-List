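; Menu navigation manager that handles keyboard, gamepad and mouse-hover focus across UI panels.
; Registered panels become indexed steps, each tracking its navigable widgets and selection through BPI_KeyboardNavigable interfaces.
; Direction and confirm keys run the action the focused widget declares: move, cycle, click, change value or custom index jump; Left/Right actions are empty stubs.
; Escape notifies panels above the focused step, otherwise the focused one, unless overridden, and dispatchers report changes.
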(fn OnInput
  (params (Key :type Key%20Structure))
  (bind _navigableitemarray_raw (Variables|AMS|Variables|GetNavigableItemArray_raw))
  (bind _currentlyfocusedstep (Variables|AMS|Variables|GetCurrentlyFocusedStep))
  (bind _output (Utilities|Array|Get(acopy) _navigableitemarray_raw _currentlyfocusedstep))
  (bind (_navigablewidgets _selectedwidgetindex) (Utilities|Struct|BreakFNavItem _output))
  (bind _output_get (LocalVariables|SettempPressedKey Key))
  (if (Utilities|Array|ContainsItem (Utilities|Array|MakeArray "Escape" "Gamepad_Special_Right") _output_get)
    (if (Variables|AMS|Variables|GetOverrideEscape)
      (Default|CallOnEscapewhenOverrideEnabled)
      (return (Class|WidgetBlueprintLibrary|Unhandled))
      (else
        (AMS|RemoveUnfocusedSteps true)
        (Default|CallOnEscape)
        (Default|CallOnSelectedItemChange)
        (return (Class|WidgetBlueprintLibrary|Handled))))
    (elif (Utilities|Array|IsValidIndex _navigableitemarray_raw _currentlyfocusedstep)
      (bind _action (Class|BPIKeyboardNavigable|GetNavigationAction(Message) (.widget (Utilities|Array|Get(acopy) _navigablewidgets _selectedwidgetindex))))
      (AMS|Navigate (LocalVariables|GettempPressedKey) (Utilities|Array|MakeArray "Up" "W" "Gamepad_DPad_Up" "Gamepad_LeftStick_Up") (.OnUp (Utilities|Struct|BreakFNavItemAction _action)) (.OnUp (Utilities|Struct|BreakFNavItemCustomAction (.CustomAction (Utilities|Struct|BreakFNavItemAction _action)))))
      (AMS|Navigate (LocalVariables|GettempPressedKey) (Utilities|Array|MakeArray "Down" "S" "Gamepad_DPad_Down" "Gamepad_LeftStick_Down") (.OnDown (Utilities|Struct|BreakFNavItemAction _action)) (.OnDown (Utilities|Struct|BreakFNavItemCustomAction (.CustomAction (Utilities|Struct|BreakFNavItemAction _action)))))
      (AMS|Navigate (LocalVariables|GettempPressedKey) (Utilities|Array|MakeArray "Right" "D" "Gamepad_DPad_Right" "Gamepad_LeftStick_Right") (.OnRight (Utilities|Struct|BreakFNavItemAction _action)) (.OnRight (Utilities|Struct|BreakFNavItemCustomAction (.CustomAction (Utilities|Struct|BreakFNavItemAction _action)))))
      (AMS|Navigate (LocalVariables|GettempPressedKey) (Utilities|Array|MakeArray "Left" "A" "Gamepad_DPad_Left" "Gamepad_LeftStick_Left") (.OnLeft (Utilities|Struct|BreakFNavItemAction _action)) (.OnLeft (Utilities|Struct|BreakFNavItemCustomAction (.CustomAction (Utilities|Struct|BreakFNavItemAction _action)))))
      (AMS|Navigate (LocalVariables|GettempPressedKey) (Utilities|Array|MakeArray "Enter" "SpaceBar" "Gamepad_FaceButton_Bottom" "E") (.OnEnter (Utilities|Struct|BreakFNavItemAction _action)) (.OnEnter (Utilities|Struct|BreakFNavItemCustomAction (.CustomAction (Utilities|Struct|BreakFNavItemAction _action))))))))

(fn AddtoNavigableArray
  (params (Nav%20Item :type F%20Nav%20Item%20Structure%20%28by%20ref%29))
  (bind (_panelreferance _navigablewidgets _selectedwidgetindex _navitemseventhandler) (Utilities|Struct|BreakFNavItem Nav%20Item))
  ;[1 1 1] Chek if the item can be navigated and add to array
  (LocalVariables|SettempIndex 0)
  (Utilities|IsValid _panelreferance
    (:Is%20Valid
      (LocalVariables|SettempPanelRef _panelreferance)
      (LocalVariables|SettempEventHandler _navitemseventhandler)
      (if (Utilities|DoesObjectImplementInterface _panelreferance "/Game/Library/Menu/MenuSystem/Widgets/Interface/BPI_KeyboardNavigablePanel.BPI_KeyboardNavigablePanel_C")
        (for _array_element _navigablewidgets
          (if (Utilities|DoesObjectImplementInterface (Utilities|Struct|BreakFWidgetFix _array_element) "/Game/Library/Menu/MenuSystem/Widgets/Interface/BPI_KeyboardNavigable.BPI_KeyboardNavigable_C")
            (Class|BPIKeyboardNavigable|SetEventHandler(Message) (Utilities|Struct|BreakFWidgetFix _array_element) (LocalVariables|GettempEventHandler))
            (Class|BPIKeyboardNavigable|SetIndex(Message) (Utilities|Struct|BreakFWidgetFix _array_element) (LocalVariables|GettempIndex) (+ (Utilities|Array|LastIndex (Variables|AMS|Variables|GetNavigableItemArray_raw)) 1))
            (EventDispatchers|BindEventtoOnMouseHover (LocalVariables|GettempEventHandler) (EventDispatchers|CreateEvent :!event NavItemMouseHover))
            (EventDispatchers|BindEventtoOnMouseUnhover (LocalVariables|GettempEventHandler) (EventDispatchers|CreateEvent :!event NavItemMouseUnhover))
            (EventDispatchers|BindEventtoOnValueChange (LocalVariables|GettempEventHandler) (EventDispatchers|CreateEvent :!event OnValueChanged))
            (Utilities|Array|AddUnique (LocalVariables|GettempWidgetArray) _array_element)
            (Math|Integer|IncrementInt (LocalVariables|GettempIndex))))
        (bind _returnvalue (Utilities|Array|Add (Variables|AMS|Variables|GetNavigableItemArray_raw) (Utilities|Struct|MakeFNavItem (LocalVariables|GettempPanelRef) (LocalVariables|GettempWidgetArray) _selectedwidgetindex (LocalVariables|GettempEventHandler))))
        (Class|BPIKeyboardNavigablePanel|SetStepIndex(Message) (LocalVariables|GettempPanelRef) _returnvalue)
        (AMS|SetNavigationFocus true _returnvalue)
        (Default|CallOnSelectedItemChange)
        (return (LocalVariables|GettempWidgetArray))))))

(fn GetNavItemsfromContainer
  (params (Box :type Widget%20Object%20Reference%20%28by%20ref%29) (Is%20Horizontal/Vertical :type Boolean))
  (if Is%20Horizontal/Vertical
    (bind _ashorizontal_box (Utilities|Casting|CastToHorizontalBox Box))
    (for _index (range 0 (- (Class|PanelWidget|GetChildrenCount _ashorizontal_box) 1))
      (Utilities|Array|Add (LocalVariables|GettempWidgetArray) (Utilities|Struct|MakeFWidgetFix (Class|PanelWidget|GetChildat _ashorizontal_box _index))))
    (else
      (bind _asvertical_box (Utilities|Casting|CastToVerticalBox Box))
      (for _index_2 (range 0 (- (Class|PanelWidget|GetChildrenCount _asvertical_box) 1))
        (Utilities|Array|Add (LocalVariables|GettempWidgetArray) (Utilities|Struct|MakeFWidgetFix (Class|PanelWidget|GetChildat _asvertical_box _index_2))))))
  (return (LocalVariables|GettempWidgetArray)))

(fn SetNavigationFocus
  (params (Focus%20Add/Clear :type Boolean) (StepIndex :type Integer))
  (bind _navigableitemarray_raw (Variables|AMS|Variables|GetNavigableItemArray_raw))
  (bind _navigableitemarray_raw_2 (Variables|AMS|Variables|GetNavigableItemArray_raw))
  (bind _output (Utilities|Array|Get(acopy) _navigableitemarray_raw StepIndex))
  (bind (_navigablewidgets _selectedwidgetindex) (Utilities|Struct|BreakFNavItem _output))
  (bind _output_2 (Utilities|Array|Get(acopy) _navigablewidgets _selectedwidgetindex))
  (bind _widget (Utilities|Struct|BreakFWidgetFix _output_2))
  (if (and (Utilities|Array|IsValidIndex _navigableitemarray_raw_2 (Variables|AMS|Variables|GetCurrentlyFocusedStep)) (!= (Variables|AMS|Variables|GetCurrentlyFocusedStep) StepIndex))
    (Class|BPIKeyboardNavigable|RemoveFocus(Message) (.widget (Utilities|Array|Get(acopy) (.navigablewidgets (Utilities|Array|Get(acopy) _navigableitemarray_raw_2 (Variables|AMS|Variables|GetCurrentlyFocusedStep))) (.selectedwidgetindex (Utilities|Array|Get(acopy) _navigableitemarray_raw_2 (Variables|AMS|Variables|GetCurrentlyFocusedStep)))))))
  (Variables|AMS|Variables|SetCurrentlyFocusedStep StepIndex)
  (if (Utilities|Array|IsValidIndex _navigableitemarray_raw StepIndex)
    (if Focus%20Add/Clear
      (Class|BPIKeyboardNavigable|SetFocus(Message) _widget)
      (else
        (Class|BPIKeyboardNavigable|RemoveFocus(Message) _widget)))))

(fn NavItemMouseHover
  (params (SelectedIndex :type Integer) (StepIndex :type Integer))
  (bind _navigableitemarray_raw (Variables|AMS|Variables|GetNavigableItemArray_raw))
  (if (Utilities|Array|IsValidIndex _navigableitemarray_raw StepIndex)
    (LocalVariables|SetNavItemChanged (or (!= (Variables|AMS|Variables|GetCurrentlyFocusedStep) StepIndex) (!= (.selectedwidgetindex (Utilities|Array|Get(acopy) (Variables|AMS|Variables|GetNavigableItemArray_raw) (Variables|AMS|Variables|GetCurrentlyFocusedStep))) SelectedIndex)))
    (AMS|SetNavigationFocus false StepIndex)
    (Utilities|Struct|SetmembersinFNavItem (Utilities|Array|Get(acopy) _navigableitemarray_raw StepIndex) SelectedIndex)
    (AMS|SetNavigationFocus true StepIndex)
    ;[1 1 1] Call OnNavigation only if the selected item changed
    (if (LocalVariables|GetNavItemChanged)
      (Default|CallOnSelectedItemChange))))

(fn NavItemMouseUnhover
  (params (selectedIndex :type Integer) (StepIndex :type Integer)))

(fn NavigateUp
  (bind _navigableitemarray_raw (Variables|AMS|Variables|GetNavigableItemArray_raw))
  (bind _currentlyfocusedstep (Variables|AMS|Variables|GetCurrentlyFocusedStep))
  (bind _output (Utilities|Array|Get(acopy) _navigableitemarray_raw _currentlyfocusedstep))
  (bind _selectedwidgetindex (Utilities|Struct|BreakFNavItem _output))
  (bind _returnvalue (- _selectedwidgetindex 1))
  (if (>= _returnvalue 0)
    (AMS|SetNavigationFocus false (Variables|AMS|Variables|GetCurrentlyFocusedStep))
    (Utilities|Struct|SetmembersinFNavItem _output _returnvalue)
    (AMS|SetNavigationFocus true (Variables|AMS|Variables|GetCurrentlyFocusedStep))
    (Default|CallOnSelectedItemChange)))

(fn NavigateDown
  (bind _navigableitemarray_raw (Variables|AMS|Variables|GetNavigableItemArray_raw))
  (bind _currentlyfocusedstep (Variables|AMS|Variables|GetCurrentlyFocusedStep))
  (bind _output (Utilities|Array|Get(acopy) _navigableitemarray_raw _currentlyfocusedstep))
  (bind (_panelreferance _navigablewidgets _selectedwidgetindex) (Utilities|Struct|BreakFNavItem _output))
  (bind _returnvalue (+ _selectedwidgetindex 1))
  (if (>= (Utilities|Array|LastIndex _navigablewidgets) _returnvalue)
    (AMS|SetNavigationFocus false (Variables|AMS|Variables|GetCurrentlyFocusedStep))
    (Utilities|Struct|SetmembersinFNavItem _output _returnvalue)
    (AMS|SetNavigationFocus true (Variables|AMS|Variables|GetCurrentlyFocusedStep))
    (Default|CallOnSelectedItemChange)))

(fn NavigateLeft)

(fn NavigateRight)

(fn Navigate
  (params (PressedKey :type Key%20Structure) (ExpectedKey :type Array%20of%20Key%20Structures) (ActionType :type ENavActionTypes%20Enum :default "NewEnumerator5") (CustomAction :type String))
  (if (Utilities|Array|ContainsItem ExpectedKey PressedKey)
    (Utilities|FlowControl|Sequence
      (:then_0
        (switch Utilities|FlowControl|Switch|SwitchonENavActionTypes ActionType
          (:NewEnumerator0
            (AMS|KeyboardNavigation|NavigateDown))
          (:NewEnumerator1
            (AMS|KeyboardNavigation|NavigateUp))
          (:NewEnumerator2
            (AMS|KeyboardNavigation|NavigateRight))
          (:NewEnumerator3
            (AMS|KeyboardNavigation|NavigateLeft))
          (:NewEnumerator4
            (AMS|KeyboardNavigation|SimulateClick))
          (:NewEnumerator6
            (AMS|KeyboardNavigation|CycleLast))
          (:NewEnumerator7
            (AMS|KeyboardNavigation|CycleFirst))
          (:NewEnumerator8
            (AMS|KeyboardNavigation|UpdateValue true))
          (:NewEnumerator9
            (AMS|KeyboardNavigation|UpdateValue false))
          (:NewEnumerator10
            (AMS|KeyboardNavigation|CustomNavigation CustomAction))))
      (:then_1
        (Default|CallOnNavigation (|GetNavigationDeviceType PressedKey))))))

(fn CycleLast
  (bind _navigableitemarray_raw (Variables|AMS|Variables|GetNavigableItemArray_raw))
  (bind _currentlyfocusedstep (Variables|AMS|Variables|GetCurrentlyFocusedStep))
  (bind _output (Utilities|Array|Get(acopy) _navigableitemarray_raw _currentlyfocusedstep))
  (AMS|SetNavigationFocus false (Variables|AMS|Variables|GetCurrentlyFocusedStep))
  (Utilities|Struct|SetmembersinFNavItem _output (Utilities|Array|LastIndex (.NavigableWidgets (Utilities|Struct|BreakFNavItem _output))))
  (AMS|SetNavigationFocus true (Variables|AMS|Variables|GetCurrentlyFocusedStep))
  (Default|CallOnSelectedItemChange))

(fn CycleFirst
  (AMS|SetNavigationFocus false (Variables|AMS|Variables|GetCurrentlyFocusedStep))
  (Utilities|Struct|SetmembersinFNavItem (Utilities|Array|Get(acopy) (Variables|AMS|Variables|GetNavigableItemArray_raw) (Variables|AMS|Variables|GetCurrentlyFocusedStep)))
  (AMS|SetNavigationFocus true (Variables|AMS|Variables|GetCurrentlyFocusedStep))
  (Default|CallOnSelectedItemChange))

(fn UpdateValue
  (params (Increase/Decrease :type Boolean))
  (bind _navigableitemarray_raw (Variables|AMS|Variables|GetNavigableItemArray_raw))
  (bind _currentlyfocusedstep (Variables|AMS|Variables|GetCurrentlyFocusedStep))
  (bind _output (Utilities|Array|Get(acopy) _navigableitemarray_raw _currentlyfocusedstep))
  (bind (_panelreferance _navigablewidgets _selectedwidgetindex) (Utilities|Struct|BreakFNavItem _output))
  (Class|BPIKeyboardNavigable|ChangeValue(Message) (Utilities|Struct|BreakFWidgetFix (Utilities|Array|Get(acopy) _navigablewidgets _selectedwidgetindex)) Increase/Decrease))

(fn SimulateClick
  (bind _navigableitemarray_raw (Variables|AMS|Variables|GetNavigableItemArray_raw))
  (bind _currentlyfocusedstep (Variables|AMS|Variables|GetCurrentlyFocusedStep))
  (bind _output (Utilities|Array|Get(acopy) _navigableitemarray_raw _currentlyfocusedstep))
  (bind (_panelreferance _navigablewidgets _selectedwidgetindex) (Utilities|Struct|BreakFNavItem _output))
  (Class|BPIKeyboardNavigable|OnClick(Message) (Utilities|Struct|BreakFWidgetFix (Utilities|Array|Get(acopy) _navigablewidgets _selectedwidgetindex))))

(fn Remove
  (params (StepIndex :type Integer) (RemoveFromArrayOnly :type Boolean))
  (bind _navigableitemarray_raw (Variables|AMS|Variables|GetNavigableItemArray_raw))
  (if RemoveFromArrayOnly
    (Utilities|Array|RemoveIndex _navigableitemarray_raw StepIndex)
    (bind _output_get (Variables|AMS|Variables|SetCurrentlyFocusedStep (Math|Integer|Clamp(Integer) (- StepIndex 1) 0 (Utilities|Array|LastIndex _navigableitemarray_raw))))
    (AMS|SetNavigationFocus true _output_get)
    (else
      (AMS|SetNavigationFocus false (Variables|AMS|Variables|GetCurrentlyFocusedStep))
      (Utilities|Array|RemoveIndex (Variables|AMS|Variables|GetNavigableItemArray_raw) StepIndex)
      (AMS|SetNavigationFocus true (Math|Integer|Clamp(Integer) (- (Variables|AMS|Variables|GetCurrentlyFocusedStep) 1) 0 (Utilities|Array|LastIndex (Variables|AMS|Variables|GetNavigableItemArray_raw)))))))

(fn SetOverrideEscape
  (params (OverrideEscape :type Boolean))
  (Variables|AMS|Variables|SetOverrideEscape OverrideEscape)
  (Default|CallOnOverrideEscape))

(fn RemoveUnfocusedSteps
  (params (EscKeyPress :type Boolean))
  (bind _navigableitemarray_raw (Variables|AMS|Variables|GetNavigableItemArray_raw))
  (bind _returnvalue (Utilities|Array|LastIndex _navigableitemarray_raw))
  (if (< _returnvalue 0) ; make sure there is atleast more than one navigable panel in the array
    (return)
    (elif (> _returnvalue (Variables|AMS|Variables|GetCurrentlyFocusedStep))
      ;[1 1 1] last step should always be the focused step. but if that is not the case, remove any higher step than the current step
      (for _index (range (+ (Variables|AMS|Variables|GetCurrentlyFocusedStep) 1) _returnvalue)
        (Class|BPIKeyboardNavigablePanel|OnEscapeInput(Message) (Utilities|Struct|BreakFNavItem (Utilities|Array|Get(acopy) (Variables|AMS|Variables|GetNavigableItemArray_raw) _index))))
      (return)
      (else
        ;[1 1 1] if player press escape key then call the on escape method on the current navigable panel
        (if EscKeyPress
          (Class|BPIKeyboardNavigablePanel|OnEscapeInput(Message) (Utilities|Struct|BreakFNavItem (Utilities|Array|Get(acopy) (Variables|AMS|Variables|GetNavigableItemArray_raw) (Variables|AMS|Variables|GetCurrentlyFocusedStep))))
          (return)
          (else
            (return)))))))

(fn GetNavigableItemList
  (return (Variables|AMS|Variables|GetNavigableItemArray_raw)))

(fn CustomNavigation
  (params (CustomAction :type String))
  (bind _output_get (LocalVariables|SettempActionParse (Utilities|String|ParseIntoArray CustomAction " ")))
  (switch int (Utilities|Array|Length _output_get)
    (:0
      (Development|PrintString 0 "No Custom navigation command is provided" true true "(R=1.000000,G=0.431695,B=0.000000,A=1.000000)") ; Reminder, in case forget to provide command
    )
    (:1
      (AMS|KeyboardNavigation|Navigateto (Math|Conversions|ToInteger(Byte) (Utilities|Array|Get(acopy) (LocalVariables|GettempActionParse)))))
    (:2
      (switch string (Utilities|Array|Get(acopy) (LocalVariables|GettempActionParse))
        (:select
          (AMS|KeyboardNavigation|Navigateto (Math|Conversions|ToInteger(Byte) (Utilities|Array|Get(acopy) (LocalVariables|GettempActionParse) 1))))))))

(fn Navigateto
  (params (index :type Integer))
  (bind _currentlyfocusedstep (Variables|AMS|Variables|GetCurrentlyFocusedStep))
  (AMS|SetNavigationFocus false _currentlyfocusedstep)
  (Utilities|Struct|SetmembersinFNavItem (Utilities|Array|Get(acopy) (Variables|AMS|Variables|GetNavigableItemArray_raw) _currentlyfocusedstep) index)
  (AMS|SetNavigationFocus true (Variables|AMS|Variables|GetCurrentlyFocusedStep))
  (Default|CallOnSelectedItemChange))

(fn GetCurrentStep
  (return (Variables|AMS|Variables|GetCurrentlyFocusedStep)))

(fn GetSelectedItem
  (bind _navigableitemarray_raw (Variables|AMS|Variables|GetNavigableItemArray_raw))
  (bind _currentlyfocusedstep (Variables|AMS|Variables|GetCurrentlyFocusedStep))
  (bind _output (Utilities|Array|Get(acopy) _navigableitemarray_raw _currentlyfocusedstep))
  (bind (_panelreferance _navigablewidgets _selectedwidgetindex) (Utilities|Struct|BreakFNavItem _output))
  (return (.widget (Utilities|Array|Get(acopy) _navigablewidgets _selectedwidgetindex))))

(fn OnValueChanged
  (params (Increase%20/%20Decrease :type Boolean))
  (Default|CallOnSelectedItemValueChange))