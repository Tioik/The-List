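; BP_Globe is a cyberpunk FX globe prop with three selectable looks: Information, Geographic and Warning.
; The construction script uses GlobeType to set the sphere and inner-layer materials and a color-matched orbit particle template.
; It shows three extra particle systems only for the Warning type.
; Tick slowly spins the sphere in relative space and both orbit effects in world space with a fixed per-frame yaw step, independent of delta time.
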(event EventTick
  (params (DeltaSeconds :type Float%20%28single-precision%29))
  (bind _orbit1 (Variables|Default|GetOrbit1))
  (bind _orbit2 (Variables|Default|GetOrbit2))
  (bind _sphere (Variables|Default|GetSphere))
  (bind _returnvalue (Transformation|GetWorldRotation _orbit2))
  (bind _returnvalue_2 (Transformation|GetWorldRotation _orbit1))
  (bind _relativerotation (Variables|/Script/Engine.SceneComponent|GetRelativeRotation _sphere))
  (Transformation|SetRelativeRotation _sphere (Math|Rotator|MakeRotator (.roll _relativerotation) (.pitch _relativerotation) (- (.yaw _relativerotation) 0.1)) false false)
  (Transformation|SetWorldRotation _orbit1 (Math|Rotator|MakeRotator (.roll _returnvalue_2) (.pitch _returnvalue_2) (- (.yaw _returnvalue_2) 0.1)) false false)
  (Transformation|SetWorldRotation _orbit2 (Math|Rotator|MakeRotator (.roll _returnvalue) (.pitch _returnvalue) (- (.yaw _returnvalue) 0.1)) false false))

(fn ConstructionScript
  (bind _inner_layer (Variables|Default|GetInner%20layer))
  (bind _sphere (Variables|Default|GetSphere))
  (bind _orbit2 (Variables|Default|GetOrbit2))
  (switch Utilities|FlowControl|Switch|SwitchonENUM_GlobeType (Variables|Default|GetGlobeType)
    (:NewEnumerator0
      (Rendering|Material|SetMaterial _sphere 0 "/Game/Library/FX/CyberPunk_FX_Pack2/Materials/Globe/M_Globe_Info.M_Globe_Info")
      (Rendering|Material|SetMaterial _inner_layer 0 "/Game/Library/FX/CyberPunk_FX_Pack2/Materials/Globe/M_Globe_Background_InfoGeo.M_Globe_Background_InfoGeo")
      (Effects|Components|ParticleSystem|SetTemplate _orbit2 "/Game/Library/FX/CyberPunk_FX_Pack2/Particles/P_Globe_Orbit_Blue.P_Globe_Orbit_Blue")
      (Rendering|SetVisibility (Variables|Default|GetParticleSystem2) false false :!label _label))
    (:NewEnumerator1
      (Rendering|Material|SetMaterial _sphere 0 "/Game/Library/FX/CyberPunk_FX_Pack2/Materials/Globe/M_Globe_Geography.M_Globe_Geography")
      (Rendering|Material|SetMaterial _inner_layer 0 "/Game/Library/FX/CyberPunk_FX_Pack2/Materials/Globe/M_Globe_Background_InfoGeo.M_Globe_Background_InfoGeo")
      (Effects|Components|ParticleSystem|SetTemplate _orbit2 "/Game/Library/FX/CyberPunk_FX_Pack2/Particles/P_Globe_Orbit_Green.P_Globe_Orbit_Green")
      (goto _label))
    (:NewEnumerator2
      (Rendering|Material|SetMaterial _sphere 0 "/Game/Library/FX/CyberPunk_FX_Pack2/Materials/Globe/M_Globe_Warning.M_Globe_Warning")
      (Rendering|Material|SetMaterial _inner_layer 0 "/Game/Library/FX/CyberPunk_FX_Pack2/Materials/Globe/M_Globe_Background_Warning.M_Globe_Background_Warning")
      (Effects|Components|ParticleSystem|SetTemplate _orbit2 "/Game/Library/FX/CyberPunk_FX_Pack2/Particles/P_Globe_Orbit_Red.P_Globe_Orbit_Red")
      (Rendering|SetVisibility (Variables|Default|GetParticleSystem1) true false))))