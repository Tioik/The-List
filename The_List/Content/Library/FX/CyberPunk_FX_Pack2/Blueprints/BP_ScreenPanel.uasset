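; Cyberpunk sci-fi screen panel prop that plays an animated power-on effect at BeginPlay.
; The construction script lays out panel, wire and display meshes from the orientation and screen-type enums, with an IsHacking option that swaps in a hacking material.
; At BeginPlay, timelines drive dynamic material parameters to animate the panel, dissolve the wireframe, fade the back panel and crosses, then randomly flicker and fade in the display.
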(event EventBeginPlay
  (bind _screenanimwire (Variables|Default|GetScreenAnimWire))
  (bind _screenanim (Variables|Default|GetScreenAnim))
  (bind _crosses (Variables|Default|GetCrosses))
  (bind _screen (Variables|Default|GetScreen))
  (bind _screenblur (Variables|Default|GetScreenBlur))
  (Utilities|FlowControl|Sequence
    (:then_0
      (Utilities|FlowControl|Sequence
        (:then_0
          (Rendering|SetVisibility (Variables|Default|GetCrosses) true false))
        (:then_1
          ;[1 1 1] Screen Panel material stuff
          (bind _returnvalue (Rendering|Material|CreateDynamicMaterialInstance _screenanimwire 0 (Rendering|Material|GetMaterial _screenanimwire 0) "None" :!class /Script/Engine.PrimitiveComponent))
          (Variables|Default|SetScreenAnim_W_DynMat _returnvalue)
          (bind _returnvalue_2 (Rendering|Material|CreateDynamicMaterialInstance _screenanim 0 (Rendering|Material|GetMaterial _screenanim 0) "None" :!class /Script/Engine.PrimitiveComponent))
          (Variables|Default|SetScreenAnim_DynMat _returnvalue_2)
          ;[1 1 1] Display material stuff
          (bind _returnvalue_3 (Rendering|Material|CreateDynamicMaterialInstance _screen 0 (Rendering|Material|GetMaterial _screen 0) "None" :!class /Script/Engine.PrimitiveComponent))
          (Variables|Default|SetScreen_DynMat _returnvalue_3)
          (bind _returnvalue_4 (Rendering|Material|CreateDynamicMaterialInstance _screenblur 0 (Rendering|Material|GetMaterial _screenblur 0) "None" :!class /Script/Engine.PrimitiveComponent))
          (Variables|Default|SetScreenBlur_DynMat _returnvalue_4)
          (bind _returnvalue_5 (Rendering|Material|CreateDynamicMaterialInstance _crosses 0 (Rendering|Material|GetMaterial _crosses 0) "None" :!class /Script/Engine.PrimitiveComponent))
          (Variables|Default|SetCrosses_DynMat _returnvalue_5))
        (:then_2
          ;[1 1 1] Set material default values
          (Rendering|Material|SetScalarParameterValue (Variables|Default|GetScreenAnim_DynMat) "Manual0 Or Auto1?" 0.0 :!class /Script/Engine.MaterialInstanceDynamic)
          (Rendering|Material|SetScalarParameterValue (Variables|Default|GetScreenAnim_W_DynMat) "Manual0 Or Auto1?" 0.0 :!class /Script/Engine.MaterialInstanceDynamic)
          (Rendering|Material|SetScalarParameterValue (Variables|Default|GetScreenBlur_DynMat) "Overall Opacity" 0.0 :!class /Script/Engine.MaterialInstanceDynamic)
          (Rendering|Material|SetScalarParameterValue (Variables|Default|GetScreen_DynMat) "Overall Opacity" 0.0 :!class /Script/Engine.MaterialInstanceDynamic)
          (Rendering|Material|SetScalarParameterValue (Variables|Default|GetScreenAnim_DynMat) "IsScanlineNeeded?" 1.0 :!class /Script/Engine.MaterialInstanceDynamic)
          (Rendering|Material|SetVectorParameterValue (Variables|Default|GetScreenAnim_DynMat) "Scanline Panning Speed" (Utilities|Struct|MakeLinearColor 0.0 0.0 0.0 0.0) :!class /Script/Engine.MaterialInstanceDynamic)
          (Rendering|Material|SetScalarParameterValue (Variables|Default|GetCrosses_DynMat) "Overall Opacity" 0.0 :!class /Script/Engine.MaterialInstanceDynamic))))
    (:then_1
      (Utilities|FlowControl|Sequence
        (:then_0
          ;[1 1 1] Animate the ScreenPanel
          (bind _newtrack_0 (Timeline|MainPanelAnim PlayFromStart)
            (:Update
              (Rendering|Material|SetScalarParameterValue (Variables|Default|GetScreenAnim_DynMat) "Anim" _newtrack_0 :!class /Script/Engine.MaterialInstanceDynamic)
              (Rendering|Material|SetScalarParameterValue (Variables|Default|GetScreenAnim_W_DynMat) "Anim" _newtrack_0 :!class /Script/Engine.MaterialInstanceDynamic))
            (:Finished
              (Utilities|FlowControl|Delay 0.1)
              (Utilities|FlowControl|Sequence
                (:then_1
                  ;[1 1 1] Fade back panel screen opacity to 0.2
                  (bind _newtrack_0_2 (Timeline|BackPanelOpacityFade PlayFromStart)
                    (:Update
                      (Rendering|Material|SetScalarParameterValue (Variables|Default|GetScreenAnim_DynMat) "Overall Opacity" _newtrack_0_2 :!class /Script/Engine.MaterialInstanceDynamic))
                    (:Finished
                      (Utilities|FlowControl|Sequence
                        (:then_1
                          (Rendering|Material|SetVectorParameterValue (Variables|Default|GetScreenAnim_DynMat) "Scanline Panning Speed" (Utilities|Struct|MakeLinearColor -0.1 0.0 0.0 0.0) :!class /Script/Engine.MaterialInstanceDynamic))
                        (:then_2
                          ;[1 1 1] Flicker 3 times
                          (Utilities|FlowControl|Delay 0.3)
                          (Rendering|Material|SetScalarParameterValue (Variables|Default|GetScreen_DynMat) "Overall Opacity" 1.0 :!class /Script/Engine.MaterialInstanceDynamic :!label _label)
                          (Utilities|FlowControl|Delay 0.05)
                          (Rendering|Material|SetScalarParameterValue (Variables|Default|GetScreen_DynMat) "Overall Opacity" 0.0 :!class /Script/Engine.MaterialInstanceDynamic)
                          (bind _result (Math|Integer|IncrementInt (Variables|Default|GetIterator))
                            (:%20%20
                              (if (< _result (Math|Random|RandomIntegerinRange 3 5))
                                (Utilities|FlowControl|Delay 0.05)
                                (goto _label)
                                (else
                                  ;[1 1 1] Fade in screen texture
                                  (Utilities|FlowControl|Delay 0.1)
                                  (bind _newtrack_1 (Timeline|ScreenFadeIn PlayFromStart)
                                    (:Update
                                      (Rendering|Material|SetScalarParameterValue (Variables|Default|GetScreen_DynMat) "Overall Opacity" _newtrack_1 :!class /Script/Engine.MaterialInstanceDynamic)
                                      (if (not (Variables|Default|GetIsHacking?))
                                        (Rendering|Material|SetScalarParameterValue (Variables|Default|GetScreenBlur_DynMat) "Overall Opacity" _newtrack_1 :!class /Script/Engine.MaterialInstanceDynamic)))))))))))))
                (:then_2
                  (bind _newtrack_0_3 (Timeline|CrossesFadeIn PlayFromStart)
                    (:Update
                      (Rendering|Material|SetScalarParameterValue (Variables|Default|GetCrosses_DynMat) "Overall Opacity" _newtrack_0_3 :!class /Script/Engine.MaterialInstanceDynamic))))))))
        (:then_1
          (Utilities|FlowControl|Delay 0.7)
          ;[1 1 1] Dissolve the wire screen
          (bind _returnvalue_6 (Rendering|Material|GetVectorParameterValue (Variables|Default|GetScreenAnim_W_DynMat) "Emissive Color" :!class /Script/Engine.MaterialInstanceDynamic))
          (bind _newtrack_0_4 (Timeline|WirepanelFade PlayFromStart)
            (:Update
              (Rendering|Material|SetVectorParameterValue (Variables|Default|GetScreenAnim_W_DynMat) "Emissive Color" (Utilities|Struct|MakeLinearColor (.R (Utilities|Struct|BreakLinearColor _returnvalue_6)) (.G (Utilities|Struct|BreakLinearColor _returnvalue_6)) (.B (Utilities|Struct|BreakLinearColor _returnvalue_6)) _newtrack_0_4) :!class /Script/Engine.MaterialInstanceDynamic))))))))

(fn ConstructionScript
  (bind _returnvalue (Transformation|GetActorScale3D))
  (bind _returnvalue_2 (Transformation|GetActorScale3D))
  (bind _screenanim (Variables|Default|GetScreenAnim))
  (bind _screenpanelrotation (LocalVariables|GetScreenPanelRotation))
  (bind _screenanimwire (Variables|Default|GetScreenAnimWire))
  (bind _screenanim_2 (Variables|Default|GetScreenAnim))
  (bind _screenanimwire_2 (Variables|Default|GetScreenAnimWire))
  (bind _screenanim_3 (Variables|Default|GetScreenAnim))
  (bind _screenanimwire_3 (Variables|Default|GetScreenAnimWire))
  (bind _screenanim_4 (Variables|Default|GetScreenAnim))
  (bind _screenanimwire_4 (Variables|Default|GetScreenAnimWire))
  (bind _screenanim_5 (Variables|Default|GetScreenAnim))
  (bind _screenanimwire_5 (Variables|Default|GetScreenAnimWire))
  (bind _screenanim_6 (Variables|Default|GetScreenAnim))
  (bind _screenanimwire_6 (Variables|Default|GetScreenAnimWire))
  (bind _screenlocations_horizontal (Variables|Default|GetScreenLocations_Horizontal))
  (bind _screenanim_7 (Variables|Default|GetScreenAnim))
  (bind _screenanimwire_7 (Variables|Default|GetScreenAnimWire))
  (bind _screenlocations_horizontal_2 (Variables|Default|GetScreenLocations_Horizontal))
  (bind _screenanim_8 (Variables|Default|GetScreenAnim))
  (bind _screenanimwire_8 (Variables|Default|GetScreenAnimWire))
  (bind _screenlocations_horizontal_3 (Variables|Default|GetScreenLocations_Horizontal))
  (bind _screenanim_9 (Variables|Default|GetScreenAnim))
  (bind _screenanimwire_9 (Variables|Default|GetScreenAnimWire))
  (bind _screenlocations_horizontal_4 (Variables|Default|GetScreenLocations_Horizontal))
  (bind _screenanim_10 (Variables|Default|GetScreenAnim))
  (bind _screenanimwire_10 (Variables|Default|GetScreenAnimWire))
  (bind _screenlocations_horizontal_5 (Variables|Default|GetScreenLocations_Horizontal))
  (bind _screenpanelrotation_2 (LocalVariables|GetScreenPanelRotation))
  (bind _screenpanelrotation_3 (LocalVariables|GetScreenPanelRotation))
  (bind _screenpanelrotation_4 (LocalVariables|GetScreenPanelRotation))
  (bind _screenpanelrotation_5 (LocalVariables|GetScreenPanelRotation))
  (bind _screenpanelrotation_6 (LocalVariables|GetScreenPanelRotation))
  (bind _screenpanelrotation_7 (LocalVariables|GetScreenPanelRotation))
  (bind _screenpanelrotation_8 (LocalVariables|GetScreenPanelRotation))
  (bind _screenpanelrotation_9 (LocalVariables|GetScreenPanelRotation))
  (bind _screenpanelrotation_10 (LocalVariables|GetScreenPanelRotation))
  (bind _screenlocations_vertical (Variables|Default|GetScreenLocations_Vertical))
  (bind _screenlocations_vertical_2 (Variables|Default|GetScreenLocations_Vertical))
  (bind _screenlocations_vertical_3 (Variables|Default|GetScreenLocations_Vertical))
  (bind _screenlocations_vertical_4 (Variables|Default|GetScreenLocations_Vertical))
  (bind _screenlocations_vertical_5 (Variables|Default|GetScreenLocations_Vertical))
  (bind _screen (Variables|Default|GetScreen))
  (bind _screen_2 (Variables|Default|GetScreen))
  (bind _output (Utilities|Array|Get(acopy) _screenlocations_vertical))
  (bind _output_2 (Utilities|Array|Get(acopy) _screenlocations_vertical_2 1))
  (bind _output_3 (Utilities|Array|Get(acopy) _screenlocations_vertical_3 2))
  (bind _output_4 (Utilities|Array|Get(acopy) _screenlocations_vertical_4 3))
  (bind _output_5 (Utilities|Array|Get(acopy) _screenlocations_vertical_5 4))
  (bind _output_6 (Utilities|Array|Get(acopy) _screenlocations_horizontal))
  (bind _output_7 (Utilities|Array|Get(acopy) _screenlocations_horizontal_2 1))
  (bind _output_8 (Utilities|Array|Get(acopy) _screenlocations_horizontal_3 2))
  (bind _output_9 (Utilities|Array|Get(acopy) _screenlocations_horizontal_4 3))
  (bind _output_10 (Utilities|Array|Get(acopy) _screenlocations_horizontal_5 4))
  (bind _relativelocation (Variables|/Script/Engine.SceneComponent|GetRelativeLocation _screen))
  (Rendering|SetVisibility (Variables|Default|GetCrosses) false false)
  (switch Utilities|FlowControl|Switch|SwitchonENUM_ScreenPanel_Type (Variables|Default|GetENUM_PanelType)
    (:NewEnumerator1
      (Utilities|FlowControl|Sequence
        (:then_0
          (Transformation|SetRelativeLocationAndRotation (Variables|Default|GetCrosses) "-0.110007,2.494553,30.308668" "-90.000000,-26.565033,116.564163" false false)
          ;[1 1 1] HORIZONTAL
          (Components|StaticMesh|SetStaticMesh (Variables|Default|GetScreenPanel) "/Game/Library/FX/CyberPunk_FX_Pack2/Meshes/Panels/SM_ScreenPanel.SM_ScreenPanel")
          (switch Utilities|FlowControl|Switch|SwitchonENUM_ScreenType (Variables|Default|GetENUM_ScreenType)
            (:NewEnumerator0
              ;[1 1 1] HORIZONTAL
              (Transformation|SetRelativeLocationAndRotation _screenanim_6 (Utilities|Array|Get(acopy) (Variables|Default|GetScreenLocations_Horizontal)) (LocalVariables|GetScreenPanelRotation) false false)
              (Components|StaticMesh|SetStaticMesh _screenanim_6 "/Game/Library/FX/CyberPunk_FX_Pack2/Meshes/Screens/SM_Screen1.SM_Screen1")
              (Components|StaticMesh|SetStaticMesh _screenanimwire_6 "/Game/Library/FX/CyberPunk_FX_Pack2/Meshes/Screens/SM_Screen1.SM_Screen1")
              (Transformation|SetRelativeLocationAndRotation _screenanimwire_6 (Math|Vector|MakeVector (.x _output_6) (+ (.y _output_6) 0.2) (.z _output_6)) (LocalVariables|GetScreenPanelRotation) false false)
              (Rendering|Material|SetMaterial _screenanimwire_6 0 "/Game/Library/FX/CyberPunk_FX_Pack2/Materials/ScreenAnimations/M_ScreenAnim_1_W.M_ScreenAnim_1_W"))
            (:NewEnumerator1
              (Transformation|SetRelativeLocationAndRotation _screenanim_7 (Utilities|Array|Get(acopy) (Variables|Default|GetScreenLocations_Horizontal) 1) (LocalVariables|GetScreenPanelRotation) false false)
              (Components|StaticMesh|SetStaticMesh _screenanim_7 "/Game/Library/FX/CyberPunk_FX_Pack2/Meshes/Screens/SM_Screen2.SM_Screen2")
              (Components|StaticMesh|SetStaticMesh _screenanimwire_7 "/Game/Library/FX/CyberPunk_FX_Pack2/Meshes/Screens/SM_Screen2.SM_Screen2")
              (Transformation|SetRelativeLocationAndRotation _screenanimwire_7 (Math|Vector|MakeVector (.x _output_7) (+ (.y _output_7) 0.2) (.z _output_7)) (LocalVariables|GetScreenPanelRotation) false false)
              (Rendering|Material|SetMaterial _screenanimwire_7 0 "/Game/Library/FX/CyberPunk_FX_Pack2/Materials/ScreenAnimations/M_ScreenAnim_2_W.M_ScreenAnim_2_W"))
            (:NewEnumerator2
              (Transformation|SetRelativeLocationAndRotation _screenanim_8 (Utilities|Array|Get(acopy) (Variables|Default|GetScreenLocations_Horizontal) 2) (LocalVariables|GetScreenPanelRotation) false false)
              (Components|StaticMesh|SetStaticMesh _screenanim_8 "/Game/Library/FX/CyberPunk_FX_Pack2/Meshes/Screens/SM_Screen3.SM_Screen3")
              (Components|StaticMesh|SetStaticMesh _screenanimwire_8 "/Game/Library/FX/CyberPunk_FX_Pack2/Meshes/Screens/SM_Screen3.SM_Screen3")
              (Transformation|SetRelativeLocationAndRotation _screenanimwire_8 (Math|Vector|MakeVector (.x _output_8) (+ (.y _output_8) 0.2) (.z _output_8)) (LocalVariables|GetScreenPanelRotation) false false)
              (Rendering|Material|SetMaterial _screenanimwire_8 0 "/Game/Library/FX/CyberPunk_FX_Pack2/Materials/ScreenAnimations/M_ScreenAnim_3_W.M_ScreenAnim_3_W"))
            (:NewEnumerator3
              (Transformation|SetRelativeLocationAndRotation _screenanim_9 (Utilities|Array|Get(acopy) (Variables|Default|GetScreenLocations_Horizontal) 3) (LocalVariables|GetScreenPanelRotation) false false)
              (Components|StaticMesh|SetStaticMesh _screenanim_9 "/Game/Library/FX/CyberPunk_FX_Pack2/Meshes/Screens/SM_Screen4.SM_Screen4")
              (Components|StaticMesh|SetStaticMesh _screenanimwire_9 "/Game/Library/FX/CyberPunk_FX_Pack2/Meshes/Screens/SM_Screen4.SM_Screen4")
              (Transformation|SetRelativeLocationAndRotation _screenanimwire_9 (Math|Vector|MakeVector (.x _output_9) (+ (.y _output_9) 0.2) (.z _output_9)) (LocalVariables|GetScreenPanelRotation) false false)
              (Rendering|Material|SetMaterial _screenanimwire_9 0 "/Game/Library/FX/CyberPunk_FX_Pack2/Materials/ScreenAnimations/M_ScreenAnim_4_W.M_ScreenAnim_4_W"))
            (:NewEnumerator4
              (Transformation|SetRelativeLocationAndRotation _screenanim_10 (Utilities|Array|Get(acopy) (Variables|Default|GetScreenLocations_Horizontal) 4) (LocalVariables|GetScreenPanelRotation) false false)
              (Components|StaticMesh|SetStaticMesh _screenanim_10 "/Game/Library/FX/CyberPunk_FX_Pack2/Meshes/Screens/SM_Screen5.SM_Screen5")
              (Components|StaticMesh|SetStaticMesh _screenanimwire_10 "/Game/Library/FX/CyberPunk_FX_Pack2/Meshes/Screens/SM_Screen5.SM_Screen5")
              (Transformation|SetRelativeLocationAndRotation _screenanimwire_10 (Math|Vector|MakeVector (.x _output_10) (+ (.y _output_10) 0.2) (.z _output_10)) (LocalVariables|GetScreenPanelRotation) false false)
              (Rendering|Material|SetMaterial _screenanimwire_10 0 "/Game/Library/FX/CyberPunk_FX_Pack2/Materials/ScreenAnimations/M_ScreenAnim_5_W.M_ScreenAnim_5_W"))))
        (:then_1
          ;[1 1 1] Re Set the screen texture location
          (Transformation|SetRelativeLocationAndRotation (Variables|Default|GetScreen) "-0.109992,3.607387,29.999996" "-90.000000, 0,90.000000" false false)
          (Transformation|SetRelativeLocationAndRotation (Variables|Default|GetScreenBlur) "-0.109992,2.107387,29.999996" "-90.000000, 0,90.000000" false false)
          ;[1 1 1] Values if TV is selected
          (if (Variables|Default|GetIsHacking?)
            (Rendering|Material|SetMaterial (Variables|Default|GetScreen) 0 "/Game/Library/FX/CyberPunk_FX_Pack2/Materials/PanelScreens/M_Hacking.M_Hacking")
            (Rendering|SetVisibility (Variables|Default|GetScreenBlur) false false)
            (Transformation|SetRelativeLocationAndRotation (Variables|Default|GetScreen) "-0.109992,1.000000,29.999996" "-90.000000, 0,90.000000" false false)
            (else
              ;[1 1 1] Re Set Values if TV is not selected
              (Rendering|Material|SetMaterial (Variables|Default|GetScreen) 0 "/Game/Library/FX/CyberPunk_FX_Pack2/Materials/PanelScreens/M_Screen1.M_Screen1")
              (Rendering|Material|SetScalarParameterValue (Variables|Default|GetScreen_DynMat) "Texture Rotation angle" 0.0 :!class /Script/Engine.MaterialInstanceDynamic))))))
    (:NewEnumerator0
      (Utilities|FlowControl|Sequence
        (:then_0
          (Transformation|SetRelativeLocationAndRotation (Variables|Default|GetCrosses) "-0.110007,2.494553,45.049564" "0.000000,179.999115,-89.999954" false false)
          ;[1 1 1] VERTICAL
          (Components|StaticMesh|SetStaticMesh (Variables|Default|GetScreenPanel) "/Game/Library/FX/CyberPunk_FX_Pack2/Meshes/Panels/SM_ScreenPanel2.SM_ScreenPanel2")
          (switch Utilities|FlowControl|Switch|SwitchonENUM_ScreenType (Variables|Default|GetENUM_ScreenType)
            (:NewEnumerator0
              ;[1 1 1] VERTICAL
              (Transformation|SetRelativeLocationAndRotation _screenanim (Utilities|Array|Get(acopy) (Variables|Default|GetScreenLocations_Vertical)) (Math|Rotator|MakeRotator (.roll _screenpanelrotation_2) (- (.pitch _screenpanelrotation_2) -9e+01) (.yaw _screenpanelrotation_2)) false false)
              (Components|StaticMesh|SetStaticMesh _screenanim "/Game/Library/FX/CyberPunk_FX_Pack2/Meshes/Screens/SM_Screen1.SM_Screen1")
              (Components|StaticMesh|SetStaticMesh _screenanimwire "/Game/Library/FX/CyberPunk_FX_Pack2/Meshes/Screens/SM_Screen1.SM_Screen1")
              (Transformation|SetRelativeLocationAndRotation _screenanimwire (Math|Vector|MakeVector (.x _output) (+ (.y _output) 0.2) (.z _output)) (Math|Rotator|MakeRotator (.roll _screenpanelrotation) (- (.pitch _screenpanelrotation) -9e+01) (.yaw _screenpanelrotation)) false false)
              (Rendering|Material|SetMaterial _screenanimwire 0 "/Game/Library/FX/CyberPunk_FX_Pack2/Materials/ScreenAnimations/M_ScreenAnim_1_W.M_ScreenAnim_1_W"))
            (:NewEnumerator1
              (Transformation|SetRelativeLocationAndRotation _screenanim_2 (Utilities|Array|Get(acopy) (Variables|Default|GetScreenLocations_Vertical) 1) (Math|Rotator|MakeRotator (.roll _screenpanelrotation_3) (- (.pitch _screenpanelrotation_3) -9e+01) (.yaw _screenpanelrotation_3)) false false)
              (Components|StaticMesh|SetStaticMesh _screenanim_2 "/Game/Library/FX/CyberPunk_FX_Pack2/Meshes/Screens/SM_Screen2.SM_Screen2")
              (Components|StaticMesh|SetStaticMesh _screenanimwire_2 "/Game/Library/FX/CyberPunk_FX_Pack2/Meshes/Screens/SM_Screen2.SM_Screen2")
              (Transformation|SetRelativeLocationAndRotation _screenanimwire_2 (Math|Vector|MakeVector (.x _output_2) (+ (.y _output_2) 0.2) (.z _output_2)) (Math|Rotator|MakeRotator (.roll _screenpanelrotation_7) (- (.pitch _screenpanelrotation_7) -9e+01) (.yaw _screenpanelrotation_7)) false false)
              (Rendering|Material|SetMaterial _screenanimwire_2 0 "/Game/Library/FX/CyberPunk_FX_Pack2/Materials/ScreenAnimations/M_ScreenAnim_2_W.M_ScreenAnim_2_W"))
            (:NewEnumerator2
              (Transformation|SetRelativeLocationAndRotation _screenanim_3 (Utilities|Array|Get(acopy) (Variables|Default|GetScreenLocations_Vertical) 2) (Math|Rotator|MakeRotator (.roll _screenpanelrotation_4) (- (.pitch _screenpanelrotation_4) -9e+01) (.yaw _screenpanelrotation_4)) false false)
              (Components|StaticMesh|SetStaticMesh _screenanim_3 "/Game/Library/FX/CyberPunk_FX_Pack2/Meshes/Screens/SM_Screen3.SM_Screen3")
              (Components|StaticMesh|SetStaticMesh _screenanimwire_3 "/Game/Library/FX/CyberPunk_FX_Pack2/Meshes/Screens/SM_Screen3.SM_Screen3")
              (Transformation|SetRelativeLocationAndRotation _screenanimwire_3 (Math|Vector|MakeVector (.x _output_3) (+ (.y _output_3) 0.2) (.z _output_3)) (Math|Rotator|MakeRotator (.roll _screenpanelrotation_8) (- (.pitch _screenpanelrotation_8) -9e+01) (.yaw _screenpanelrotation_8)) false false)
              (Rendering|Material|SetMaterial _screenanimwire_3 0 "/Game/Library/FX/CyberPunk_FX_Pack2/Materials/ScreenAnimations/M_ScreenAnim_3_W.M_ScreenAnim_3_W"))
            (:NewEnumerator3
              (Transformation|SetRelativeLocationAndRotation _screenanim_4 (Utilities|Array|Get(acopy) (Variables|Default|GetScreenLocations_Vertical) 3) (Math|Rotator|MakeRotator (.roll _screenpanelrotation_5) (- (.pitch _screenpanelrotation_5) -9e+01) (.yaw _screenpanelrotation_5)) false false)
              (Components|StaticMesh|SetStaticMesh _screenanim_4 "/Game/Library/FX/CyberPunk_FX_Pack2/Meshes/Screens/SM_Screen4.SM_Screen4")
              (Components|StaticMesh|SetStaticMesh _screenanimwire_4 "/Game/Library/FX/CyberPunk_FX_Pack2/Meshes/Screens/SM_Screen4.SM_Screen4")
              (Transformation|SetRelativeLocationAndRotation _screenanimwire_4 (Math|Vector|MakeVector (.x _output_4) (+ (.y _output_4) 0.2) (.z _output_4)) (Math|Rotator|MakeRotator (.roll _screenpanelrotation_9) (- (.pitch _screenpanelrotation_9) -9e+01) (.yaw _screenpanelrotation_9)) false false)
              (Rendering|Material|SetMaterial _screenanimwire_4 0 "/Game/Library/FX/CyberPunk_FX_Pack2/Materials/ScreenAnimations/M_ScreenAnim_4_W.M_ScreenAnim_4_W"))
            (:NewEnumerator4
              (Transformation|SetRelativeLocationAndRotation _screenanim_5 (Utilities|Array|Get(acopy) (Variables|Default|GetScreenLocations_Vertical) 4) (Math|Rotator|MakeRotator (.roll _screenpanelrotation_6) (- (.pitch _screenpanelrotation_6) -9e+01) (.yaw _screenpanelrotation_6)) false false)
              (Components|StaticMesh|SetStaticMesh _screenanim_5 "/Game/Library/FX/CyberPunk_FX_Pack2/Meshes/Screens/SM_Screen5.SM_Screen5")
              (Components|StaticMesh|SetStaticMesh _screenanimwire_5 "/Game/Library/FX/CyberPunk_FX_Pack2/Meshes/Screens/SM_Screen5.SM_Screen5")
              (Transformation|SetRelativeLocationAndRotation _screenanimwire_5 (Math|Vector|MakeVector (.x _output_5) (+ (.y _output_5) 0.2) (.z _output_5)) (Math|Rotator|MakeRotator (.roll _screenpanelrotation_10) (- (.pitch _screenpanelrotation_10) -9e+01) (.yaw _screenpanelrotation_10)) false false)
              (Rendering|Material|SetMaterial _screenanimwire_5 0 "/Game/Library/FX/CyberPunk_FX_Pack2/Materials/ScreenAnimations/M_ScreenAnim_5_W.M_ScreenAnim_5_W"))))
        (:then_1
          ;[1 1 1] Re Set the screen texture location
          (Transformation|SetRelativeLocationAndRotation (Variables|Default|GetScreen) "-0.109992,3.607387,46.477528" "0.000000,-180.000000,-90.000000" false false)
          (Transformation|SetRelativeLocationAndRotation (Variables|Default|GetScreenBlur) "-0.109992,2.107387,46.477528" "0.000000,-180.000000,-90.000000" false false)
          ;[1 1 1] Values if TV is selected
          (if (Variables|Default|GetIsHacking?)
            (Rendering|Material|SetMaterial _screen 0 "/Game/Library/FX/CyberPunk_FX_Pack2/Materials/PanelScreens/M_Hacking.M_Hacking")
            (Rendering|SetVisibility (Variables|Default|GetScreenBlur) false false)
            (Transformation|SetWorldScale3D _screen (Math|Vector|MakeVector (/ (.x _returnvalue_2) 1.25) (/ (.y _returnvalue_2) 2.0) (.z _returnvalue_2)))
            (Transformation|SetRelativeRotation _screen "-90.000000,0.000000,90.000000" false false)
            (Transformation|SetRelativeLocation _screen (Math|Vector|MakeVector (.x _relativelocation) (- (.y _relativelocation) 1.5) (- (.z _relativelocation) 1.0)) false false)
            (else
              ;[1 1 1] Re Set Values if TV is not selected
              (Rendering|Material|SetMaterial _screen_2 0 "/Game/Library/FX/CyberPunk_FX_Pack2/Materials/PanelScreens/M_Screen1.M_Screen1")
              (Transformation|SetWorldScale3D _screen_2 (Math|Vector|MakeVector (/ (.x _returnvalue) 1.93) (/ (.y _returnvalue) 1.23) (.z _returnvalue))))))))))