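; BP_HoloTable is a holographic table effect that reveals a miniature city with three targets when SpawnCity is called.
; It hides the city and targets, shows a flattened wireframe city, then after a delay grows the wireframe's height by timeline up to the actor's Z scale.
; The solid city then appears, a second timeline animates the wireframe's "Op" material parameter through a dynamic instance, and finally the targets become visible.
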(event Custom|Spawn%20City
  (bind _citywire (Variables|Default|GetCityWire))
  (bind _citywire_2 (Variables|Default|GetCityWire))
  (bind _relativescale3d (Variables|/Script/Engine.SceneComponent|GetRelativeScale3D _citywire_2))
  (Rendering|SetVisibility (Variables|Default|GetCity) false false)
  (Transformation|SetRelativeScale3D _citywire_2 (Math|Vector|MakeVector (.x _relativescale3d) (.y _relativescale3d) 0.0))
  (Rendering|SetVisibility _citywire_2 true false)
  (Rendering|SetVisibility (Variables|Default|GetTarget2) false false)
  (Utilities|FlowControl|Delay 2.5)
  (Variables|Default|SetCurrent%20City%20Height (.z (Transformation|GetActorScale3D)))
  (bind _newtrack_0 (Timeline|Timeline_0 PlayFromStart)
    (:Update
      (Transformation|SetWorldScale3D (Variables|Default|GetCityWire) (Math|Vector|MakeVector (Variables|Default|GetCurrent%20City%20Height) (Variables|Default|GetCurrent%20City%20Height) (* _newtrack_0 (Variables|Default|GetCurrent%20City%20Height)))))
    (:Finished
      (Rendering|SetVisibility (Variables|Default|GetCity) true false)
      (Utilities|FlowControl|Delay 0.3)
      (bind _returnvalue (Rendering|Material|CreateDynamicMaterialInstance _citywire 0 (Rendering|Material|GetMaterial _citywire 0) "None" :!class /Script/Engine.PrimitiveComponent))
      (bind _newtrack_2 (Timeline|Timeline_1 PlayFromStart)
        (:Update
          (Rendering|Material|SetScalarParameterValue _returnvalue "Op" _newtrack_2 :!class /Script/Engine.MaterialInstanceDynamic))
        (:Finished
          (Rendering|SetVisibility (Variables|Default|GetTarget2) true false))))))

(event EventBeginPlay)

(event Collision|EventActorBeginOverlap
  (params (OtherActor :type Actor%20Object%20Reference)))

(event EventTick
  (params (DeltaSeconds :type Float%20%28single-precision%29)))

(fn ConstructionScript)